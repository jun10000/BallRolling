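; Blueprint function library of shared helpers for the game's Blueprints.
; Typed getters cast the player controller, game mode and game instance, printing a red error on failure; widget and timer lookups go through the game mode.
; Other utilities cover zero-padded strings, rotator clamping, actor validity, integer-array conversion and Niagara spawning.
; Timespans format as signed minutes:seconds.centiseconds, built from an absolute value plus a negative flag.
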(fn `Absolute (Timespan)`
  (params (InTimespan :type "Timespan Structure"))
  (returns (ReturnValue :type "Timespan Structure") (IsNegative :type Boolean))
  (bind (_days _hours _minutes _seconds _milliseconds) (`KismetMathLibrary.BreakTimespan` InTimespan))
  (return (`KismetMathLibrary.MakeTimespan` (`KismetMathLibrary.Abs_Int` _days) (`KismetMathLibrary.Abs_Int` _hours) (`KismetMathLibrary.Abs_Int` _minutes) (`KismetMathLibrary.Abs_Int` _seconds) (`KismetMathLibrary.Abs_Int` _milliseconds)) (or (< _days 0) (< _hours 0) (< _minutes 0) (< _seconds 0) (< _milliseconds 0))))

(fn `ClampRotator`
  (params (Rotator :type "Rotator Structure") (XDegreeMin :type "Float (double-precision)") (XDegreeMax :type "Float (double-precision)") (YDegreeMin :type "Float (double-precision)") (YDegreeMax :type "Float (double-precision)") (ZDegreeMin :type "Float (double-precision)") (ZDegreeMax :type "Float (double-precision)"))
  (returns (ReturnValue :type "Rotator Structure"))
  (return (`KismetMathLibrary.MakeRotator` (`KismetMathLibrary.ClampAngle` (.roll Rotator) XDegreeMin XDegreeMax) (`KismetMathLibrary.ClampAngle` (.pitch Rotator) YDegreeMin YDegreeMax) (`KismetMathLibrary.ClampAngle` (.yaw Rotator) ZDegreeMin ZDegreeMax))))

(fn `GetMyGameInstance`
  (returns (GameInstance :type "/Game/Blueprints/BP_GameInstance Object Reference"))
  (bind _asbp_game_instance (cast `/Game/Blueprints/BP_GameInstance` (`GameplayStatics.GetGameInstance` null))
    (:`then`
      (return _asbp_game_instance))
    (:`CastFailed`
      (`self.PrintError` "Failed cast to BP_GameInstance"))))

(fn `GetMyGameMode`
  (returns (GameMode :type "/Game/Blueprints/BP_GameMode Object Reference"))
  (bind _asbp_game_mode (cast `/Game/Blueprints/BP_GameMode` (`GameplayStatics.GetGameMode` null))
    (:`then`
      (return _asbp_game_mode))
    (:`CastFailed`
      (`self.PrintError` "Failed cast to BP_GameMode"))))

(fn `GetMyPlayerController`
  (returns (PlayerController :type "/Game/Blueprints/BP_PlayerController Object Reference"))
  (bind _asbp_player_controller (cast `/Game/Blueprints/BP_PlayerController` (`GameplayStatics.GetPlayerController` null))
    (:`then`
      (return _asbp_player_controller))
    (:`CastFailed`
      (`self.PrintError` "Failed cast to BP_PlayerController"))))

(fn `GetRepeatedString`
  (params (String :type String) (Count :type Integer :default 1))
  (returns (ReturnValue :type String))
  (locals (CurrentString :type String))
  (for _ (range Count)
    (set `local.CurrentString` (`KismetStringLibrary.Concat_StrStr` (`local.CurrentString`) String)))
  (return (`local.CurrentString`)))

(fn `GetTimer`
  (returns (Timer :type "/Game/Blueprints/BP_Timer Object Reference"))
  (return (`/Game/Blueprints/BP_GameMode.GetTimer` (`self.GetMyGameMode` null))))

(fn `GetWidget`
  (params (Class :type "/Game/Widgets/W_Base Class Reference"))
  (returns (ReturnValue :type "/Game/Widgets/W_Base Object Reference"))
  (return (`/Game/Blueprints/BP_GameMode.GetWidget` (`self.GetMyGameMode` null) Class)))

(fn `GetZeroFilledString`
  (params (Integer :type Integer) (Digit :type Integer :default 2))
  (returns (String :type String))
  (return (`KismetStringLibrary.Right` (`KismetStringLibrary.Concat_StrStr` (`self.GetRepeatedString` "0" (- Digit 1)) (`KismetStringLibrary.Conv_IntToString` Integer)) Digit)))

(fn `IsActorValid`
  (params (InputActor :type "Actor Object Reference"))
  (returns (ReturnValue :type Boolean))
  (`/Engine/EditorBlueprintResources/StandardMacros.IsValid` InputActor
    (:`Is Valid`
      (if (`Actor.IsActorBeingDestroyed` InputActor)
        _
        (else
          (return true))))
    (:`Is Not Valid`
      _))
  (return false))

(fn `PlayParticle`
  (params (Particle :type "NiagaraSystem Object Reference") (Location :type "Vector Structure"))
  (`NiagaraFunctionLibrary.SpawnSystemAtLocation` null Particle Location))

(fn `PrintError`
  (params (Message :type String))
  (`KismetSystemLibrary.PrintString` null (`KismetStringLibrary.Concat_StrStr` "Error: " Message) true true (struct :`R` 1.0 :`A` 1.0)))

(fn `ToString (Timespan)`
  (params (InTimespan :type "Timespan Structure"))
  (returns (ReturnValue :type String))
  (bind (_returnvalue _isnegative) (`self.Absolute (Timespan)` InTimespan))
  (return (`KismetStringLibrary.Concat_StrStr` (`KismetMathLibrary.SelectString` "-" "" _isnegative) (`KismetStringLibrary.Conv_IntToString` (`KismetMathLibrary.FTrunc` (`KismetMathLibrary.GetTotalMinutes` _returnvalue))) ":" (`self.GetZeroFilledString` (`KismetMathLibrary.GetSeconds` _returnvalue)) "." (`KismetStringLibrary.Left` (`self.GetZeroFilledString` (`KismetMathLibrary.GetMilliseconds` _returnvalue) 3) 2))))

(fn `ToStringArray (IntegerArray)`
  (params (IntegerArray :type "Array of Integer"))
  (returns (StringArray :type "Array of String"))
  (locals (LocalStringArray :type "Array of String"))
  (for _array_element IntegerArray
    (`KismetArrayLibrary.Array_Add` (`local.LocalStringArray`) (`KismetStringLibrary.Conv_IntToString` _array_element)))
  (return (`local.LocalStringArray`)))