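; Goal volume actor that detects when a BP_BallActor enters its trigger and runs the goal sequence.
; On overlap it switches the player controller's input mode, stops the ball's simulation, plays its goal particle, changes the BGM and calls OnGoal with the ball.
; The construction script derives the trigger's relative scale from the cube's world size, shrinking it by twice the ball diameter with a minimum-size clamp per axis.
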(event `self.GoalTrigger.OnComponentBeginOverlap`
  (params (OverlappedComponent :type "PrimitiveComponent Object Reference") (OtherActor :type "Actor Object Reference") (OtherComp :type "PrimitiveComponent Object Reference") (OtherBodyIndex :type Integer) (bFromSweep :type Boolean) (SweepResult :type "HitResult Structure (by ref)"))
  (bind _asbp_ball_actor (cast `/Game/Blueprints/BP_BallActor` OtherActor))
  (`/Game/Blueprints/BP_PlayerController.SetInputMode` (`/Game/Blueprints/BP_FunctionLibrary.GetMyPlayerController`) "NewEnumerator2")
  (`/Game/Blueprints/BP_BallActor.SetSimulationEnable` _asbp_ball_actor false)
  (`/Game/Blueprints/BP_BallActor.PlayGoalParticle` _asbp_ball_actor)
  (`/Game/Blueprints/BP_GameMode.SetBGM` (`/Game/Blueprints/BP_FunctionLibrary.GetMyGameMode`) "/Game/Sounds/SC_気分はウイスキー.SC_気分はウイスキー" 1)
  (`self.OnGoal` _asbp_ball_actor))

(fn `UserConstructionScript`
  (bind _returnvalue (* (`SceneComponent.K2_GetComponentScale` (`self.Cube`)) (`KismetMathLibrary.MakeVector` 100.0 100.0 100.0)))
  (bind _x (.x (- _returnvalue (200.0 200.0 200.0))))
  (bind _y (.y (- _returnvalue (200.0 200.0 200.0))))
  (bind _z (.z (- _returnvalue (200.0 200.0 200.0))))
  (`SceneComponent.SetRelativeScale3D` (`self.GoalTrigger`) (/ (`KismetMathLibrary.MakeVector` (`KismetMathLibrary.SelectFloat` 1.0 _x (< _x 1.0)) (`KismetMathLibrary.SelectFloat` 1.0 _y (< _y 1.0)) (`KismetMathLibrary.SelectFloat` 1.0 _z (< _z 1.0))) _returnvalue)))