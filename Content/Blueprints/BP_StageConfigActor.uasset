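; Stage config actor that runs the flow of a ball stage from per-sub-stage settings looked up by the game mode's sub-stage index.
; InitStage sets camera, stage and BGM, plays an optional intro sequence, then spawns the ball, shows the HUD, starts the timer and binds the goal.
; On goal it pauses the timer, plays the goal sequence and results screen, then the end sequence, which opens the next stage.
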(event `InitStage`
  (bind (_returnvalue_stageindex _returnvalue_substageindex) (break `/Game/Blueprints/BP_StageIndexStruct` (`/Game/Blueprints/BP_GameMode.GetStageIndex` (`/Game/Blueprints/BP_FunctionLibrary.GetMyGameMode`))))
  (bind (_value _returnvalue) (`BlueprintMapLibrary.Map_Find` (`self.SubStageConfigs`) _returnvalue_substageindex))
  (bind (_stageactor _stagecameraactor _startballspawner _goalactor _bgm _bgm_id _bgm_part _lsactor_start _lsactor_goal _lsactor_end _nextstageindex) (break `/Game/Blueprints/BP_SubStageConfigStruct` _value))
  (if _returnvalue
    (`/Game/Blueprints/BP_PlayerController.Init` (`/Game/Blueprints/BP_FunctionLibrary.GetMyPlayerController`) _stagecameraactor _stageactor)
    (`/Game/Blueprints/BP_GameMode.SetBGM` :`self` (`/Game/Blueprints/BP_FunctionLibrary.GetMyGameMode`) :`BGM` _bgm :`ID` _bgm_id :`Part` _bgm_part)
    (`/Game/Blueprints/BP_ActorMacroLibrary.IsActorValid` _lsactor_start
      (:`IsValid`
        (`/Game/Blueprints/BP_FunctionLibrary.PlayLevelSequence` _lsactor_start (delegate `LSActor_Start_OnComplete`)))
      (:`IsNotValid`
        (`/Game/Blueprints/BP_ActorMacroLibrary.IsActorValid` _startballspawner :!label _label
          (:`IsValid`
            (`/Game/Blueprints/BP_BallSpawner.SpawnWithRespawnProcess` _startballspawner)
            (`/Game/Widgets/W_Base.PlayMainAnimation` :`self` (`/Game/Blueprints/BP_FunctionLibrary.GetWidget` "/Game/Widgets/W_HUD.W_HUD_C"))
            (`/Game/Blueprints/BP_Timer.Start` (`/Game/Blueprints/BP_FunctionLibrary.GetTimer`) true)
            (`/Game/Blueprints/BP_ActorMacroLibrary.IsActorValid` _goalactor
              (:`IsValid`
                (clear `/Game/Blueprints/BP_Goal_BaseActor.OnGoal` _goalactor)
                (add `/Game/Blueprints/BP_Goal_BaseActor.OnGoal` _goalactor (delegate `GoalActor_OnGoal`))))))))))

(event `LSActor_Start_OnComplete`
  (goto _label))

(event `GoalActor_OnGoal`
  (params (BallActor :type "/Game/Blueprints/BP_BallActor Object Reference"))
  (bind (_returnvalue_stageindex _returnvalue_substageindex) (break `/Game/Blueprints/BP_StageIndexStruct` (`/Game/Blueprints/BP_GameMode.GetStageIndex` (`/Game/Blueprints/BP_FunctionLibrary.GetMyGameMode`))))
  (bind (_stageactor _stagecameraactor _startballspawner _goalactor _bgm _bgm_id _bgm_part _lsactor_start _lsactor_goal _lsactor_end _nextstageindex) (break `/Game/Blueprints/BP_SubStageConfigStruct` (`BlueprintMapLibrary.Map_Find` (`self.SubStageConfigs`) _returnvalue_substageindex)))
  (`/Game/Blueprints/BP_Timer.Pause` (`/Game/Blueprints/BP_FunctionLibrary.GetTimer`))
  (`/Game/Blueprints/BP_ActorMacroLibrary.IsActorValid` _lsactor_goal
    (:`IsValid`
      (`/Game/Widgets/W_Base.PlayMainAnimation` :`self` (`/Game/Blueprints/BP_FunctionLibrary.GetWidget` "/Game/Widgets/W_HUD.W_HUD_C") :`IsReverse` true)
      (`/Game/Blueprints/BP_FunctionLibrary.PlayLevelSequence` _lsactor_goal (delegate `LSActor_Goal_OnComplete`)))
    (:`IsNotValid`
      (`/Game/Blueprints/BP_ActorMacroLibrary.IsActorValid` _lsactor_end :!label _label_2
        (:`IsValid`
          (`/Game/Blueprints/BP_FunctionLibrary.PlayLevelSequence` _lsactor_end (delegate `LSActor_End_OnComplete`)))
        (:`IsNotValid`
          (`KismetSystemLibrary.PrintString` "Goal!" true true (struct :`R` 1.0 :`A` 1.0)))))))

(event `LSActor_Goal_OnComplete`
  (`/Game/Widgets/W_Result.ShowResult` (cast `/Game/Widgets/W_Result` (`/Game/Blueprints/BP_FunctionLibrary.GetWidget` "/Game/Widgets/W_Result.W_Result_C") :!pure true) 0 (delegate `W_Result_OnFinish`)))

(event `W_Result_OnFinish`
  (goto _label_2))

(event `LSActor_End_OnComplete`
  (bind (_returnvalue_stageindex _returnvalue_substageindex) (break `/Game/Blueprints/BP_StageIndexStruct` (`/Game/Blueprints/BP_GameMode.GetStageIndex` (`/Game/Blueprints/BP_FunctionLibrary.GetMyGameMode`))))
  (`/Game/Blueprints/BP_GameMode.OpenStage` (`/Game/Blueprints/BP_FunctionLibrary.GetMyGameMode`) (`.NextStageIndex_40_071534F84BBE0AE9B81856A7A0502C4D` (break `/Game/Blueprints/BP_SubStageConfigStruct` (`BlueprintMapLibrary.Map_Find` (`self.SubStageConfigs`) _returnvalue_substageindex)))))

(fn `UserConstructionScript`)