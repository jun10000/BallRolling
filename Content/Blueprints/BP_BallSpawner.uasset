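; Spawner actor that creates balls at its own transform and replaces them when destroyed, apparently for a block-breaker game.
; Spawn creates a BP_BallActor and registers it through the player controller's AddBall, which decides success but leaves a rejected ball in place.
; SpawnWithRespawnProcess binds each successful ball's OnEndPlay.
; Only a Destroyed end-play reason plays a sound and spawns a rebound replacement, continuing the respawn chain.
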(event `self.ReceiveBeginPlay`)

(event `SpawnWithRespawnProcess`
  (bind (_issuccess _ballactor) (`self.Spawn`))
  (if _issuccess
    (add `self.OnEndPlay` _ballactor (delegate `Event_BallActor_EndPlay`))))

(event `Event_BallActor_EndPlay` :!signature `self.OnEndPlay`
  (params (Actor :type "Actor Object Reference") (EndPlayReason :type "EEndPlayReason Enum" :default "Destroyed"))
  (switch `EEndPlayReason` EndPlayReason
    (:`Destroyed`
      (`GameplayStatics.PlaySound2D` "/Game/Sounds/SC_ブロック崩し.SC_ブロック崩し" 1.0 1.0 0.0 null null)
      (bind (_issuccess _ballactor) (`self.Spawn`))
      (if _issuccess
        (add `self.OnEndPlay` _ballactor (delegate `Event_BallActor_EndPlay`))))))

(fn `Spawn`
  (returns (IsSuccess :type Boolean) (BallActor :type "/Game/Blueprints/BP_BallActor Object Reference"))
  (bind _returnvalue (`|SpawnActorFromClass` "/Game/Blueprints/BP_BallActor.BP_BallActor_C" (`self.GetTransform`) "Undefined" "MultiplyWithRoot" null null))
  (bind _issuccess (`/Game/Blueprints/BP_PlayerController.AddBall` (`/Game/Blueprints/BP_FunctionLibrary.GetMyPlayerController`) _returnvalue))
  (if _issuccess
    (return true _returnvalue)
    (else
      (return false null))))

(fn `UserConstructionScript`)