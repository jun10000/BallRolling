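; BP_TimerSpawner is a spawner actor that places a BP_TimerActor at its own transform.
; The construction script sets its X and Y scale from DiameterScale, keeping Z at 1.
; Spawn creates a timer actor only when the tracked one is invalid, then attaches it to the spawner's attach parent with KeepRelative rules.
; The event graph is empty, so nothing in this Blueprint calls Spawn.
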(fn `Spawn`
  (if (not (`/Game/Blueprints/BP_FunctionLibrary.IsActorValid` (`self.CurrentSpawnedActor`)))
    (bind _returnvalue (`|SpawnActorFromClass` "/Game/Blueprints/BP_TimerActor.BP_TimerActor_C" (`self.GetTransform`) "Undefined" "MultiplyWithRoot" null null))
    (`self.K2_AttachToActor` _returnvalue (`self.GetAttachParentActor`) "None" "KeepRelative" "KeepRelative" "KeepRelative" true)
    (set `self.CurrentSpawnedActor` _returnvalue)))

(fn `UserConstructionScript`
  (bind _diameterscale (`self.DiameterScale`))
  (`self.SetActorScale3D` (`KismetMathLibrary.MakeVector` _diameterscale _diameterscale 1.0)))