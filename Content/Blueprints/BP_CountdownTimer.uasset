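; BP_CountdownTimer is a countdown timer with Start, Pause, Resume and Reset, gated by a Stopping, Running or Pausing mode.
; It stores a target date-time while running and the remaining timespan while paused, so it needs no tick.
; GetTime derives the remaining time and, once it passes zero, fires and unbinds the finish callback, so completion is only detected when polled.
; Mode stays Running after expiry until Reset.
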(fn `GetTime`
  (returns (Time :type "Timespan Structure"))
  (locals (CurrentRemainingTime :type "Timespan Structure"))
  (switch `/Game/Blueprints/BP_TimerStateEnum` (`self.Mode`)
    (:`NewEnumerator0`
      (return (`self.OriginalRemainingTime`)))
    (:`NewEnumerator1`
      (bind _output_get (set `local.CurrentRemainingTime` (- (`self.TargetDTime`) (`KismetMathLibrary.Now`))))
      (if (< (`KismetMathLibrary.GetTotalMilliseconds` _output_get) 0.0)
        (`self.OnCountdownFinished`)
        (clear `self.OnCountdownFinished`)
        (return (`KismetMathLibrary.TimespanZeroValue`))
        (else
          (return (`local.CurrentRemainingTime`)))))
    (:`NewEnumerator2`
      (return (`self.RemainingTime`)))))

(fn `Pause`
  (switch `/Game/Blueprints/BP_TimerStateEnum` (`self.Mode`)
    (:`NewEnumerator1`
      (set `self.RemainingTime` (- (`self.TargetDTime`) (`KismetMathLibrary.Now`)))
      (set `self.Mode` "NewEnumerator2"))))

(fn `Reset`
  (switch `/Game/Blueprints/BP_TimerStateEnum` (`self.Mode`)
    (:`NewEnumerator1`
      _)
    (:`NewEnumerator2`
      _))
  (set `self.Mode` "NewEnumerator0"))

(fn `Resume`
  (switch `/Game/Blueprints/BP_TimerStateEnum` (`self.Mode`)
    (:`NewEnumerator2`
      (set `self.TargetDTime` (+ (`KismetMathLibrary.Now`) (`self.RemainingTime`)))
      (set `self.Mode` "NewEnumerator1"))))

(fn `Start`
  (params (Time :type "Timespan Structure") (OnFinish :type "Delegate (by ref)"))
  (switch `/Game/Blueprints/BP_TimerStateEnum` (`self.Mode`)
    (:`NewEnumerator0`
      (set `self.OriginalRemainingTime` Time)
      (set `self.TargetDTime` (+ (`KismetMathLibrary.Now`) Time))
      (clear `self.OnCountdownFinished`)
      (add `self.OnCountdownFinished` OnFinish)
      (set `self.Mode` "NewEnumerator1"))))