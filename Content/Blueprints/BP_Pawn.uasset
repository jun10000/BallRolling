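; A pawn for what appears to be a ball-on-tilting-stage game, owning both the stage and the ball.
; BeginPlay spawns the stage at the origin, then spawns the ball above it after a short delay.
; TiltStage combines an incoming rotator with the stage's current rotation, clamps X and Y within StageTiltLimit, and applies it with sweep.
; No caller or input binding for TiltStage appears here.
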(event `self.ReceiveBeginPlay`
  (`|ExecutionSequence`
    (:`then_0`
      (bind _returnvalue (`|SpawnActorFromClass` "/Game/Blueprints/BP_Stage01Actor.BP_Stage01Actor_C" (`KismetMathLibrary.MakeTransform` (0.0 0.0 0.0)) "Undefined" "MultiplyWithRoot" null null))
      (set `self.StageActor` _returnvalue))
    (:`then_1`
      (`KismetSystemLibrary.Delay` 1.0)
      (bind _returnvalue_2 (`|SpawnActorFromClass` "/Game/Blueprints/BP_BallActor.BP_BallActor_C" (`KismetMathLibrary.MakeTransform` (0.0 0.0 100.0)) "Undefined" "MultiplyWithRoot" null null))
      (set `self.BallActor` _returnvalue_2))))

(fn `Tilt Stage`
  (params (AddRotator :type "Rotator Structure"))
  (bind _stagetiltlimit (`self.StageTiltLimit`))
  (bind _stageactor (`self.StageActor`))
  (bind _returnvalue (* _stagetiltlimit -1.0))
  (`/Engine/EditorBlueprintResources/StandardMacros.IsValid` _stageactor
    (:`Is Valid`
      (`self.K2_SetActorRelativeRotation` _stageactor (`/Game/Blueprints/BP_FunctionLibrary.ClampRotator` (`KismetMathLibrary.ComposeRotators` (`self.K2_GetActorRotation` _stageactor) AddRotator) _returnvalue _stagetiltlimit _returnvalue _stagetiltlimit) true false))))

(fn `UserConstructionScript`)