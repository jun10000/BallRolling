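; BP_Spawner is a placeable spawner that creates one actor of a configurable class at its own transform, on BeginPlay or through the Trig event.
; Trig spawns only while the previously spawned actor is invalid, so one instance exists at a time.
; The new actor receives the configured tags and can optionally attach to the spawner's parent actor, keeping world transform.
; The construction script sets the view mesh from a configurable static mesh.
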(event `self.ReceiveBeginPlay`
  (if (`self.SpawnOnStartup`)
    (`/Game/Blueprints/IF_Triggerable.Trig`)))

(event `/Game/Blueprints/IF_Triggerable.Trig`
  (`/Game/Blueprints/BP_ActorMacroLibrary.IsActorValid` (`self.SpawnedActor`)
    (:`IsNotValid`
      (bind _returnvalue (`self.Spawn`))
      (bind _output_get (set `self.SpawnedActor` _returnvalue))
      (set `Actor.Tags` (`self.SpawnActorTags`) _output_get)
      (if (`self.HasSpawnedActorParent`)
        (`self.K2_AttachToActor` _output_get (`self.GetAttachParentActor`) "None" "KeepWorld" "KeepWorld" "KeepWorld" true)))))

(fn `Spawn`
  (returns (ReturnValue :type "Actor Object Reference"))
  (bind _returnvalue (`|SpawnActorFromClass` (`self.SpawnActorClass`) (`self.GetTransform`) "Undefined" "MultiplyWithRoot" null null))
  (return _returnvalue))

(fn `UserConstructionScript`
  (`StaticMeshComponent.SetStaticMesh` (`self.ViewMesh`) (`self.ViewSM`)))