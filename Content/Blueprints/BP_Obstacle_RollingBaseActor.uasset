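; BP_Obstacle_RollingBaseActor is an obstacle actor, named as a base, that spins continuously around one configurable axis.
; The construction script sets the RotatingMovement component's rotation rate from RotationAxis (None, X, Y or Z), mapping the speed to roll, pitch or yaw.
; IsReverse flips the sign of RotationSpeed, and None yields no rotation.
; The event graph holds only disabled placeholder events, so the component alone drives the motion.
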(fn `UserConstructionScript`
  (bind _returnvalue (* (`self.RotationSpeed`) (`KismetMathLibrary.SelectFloat` -1.0 1.0 (`self.IsReverse`))))
  (set `RotatingMovementComponent.RotationRate` (select `EAxis` (`self.RotationAxis`) :`X` (`KismetMathLibrary.MakeRotator` _returnvalue) :`Y` (`KismetMathLibrary.MakeRotator` 0.0 _returnvalue) :`Z` (`KismetMathLibrary.MakeRotator` 0.0 0.0 _returnvalue)) (`self.RotatingMovement`)))