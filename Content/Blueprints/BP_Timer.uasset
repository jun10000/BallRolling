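; BP_Timer is a stopwatch that measures elapsed time and can be started, paused, resumed and stopped.
; A three-state variable (Stopping, Running, Pausing) gates each function, storing a start timestamp and the time accumulated at pause.
; Resuming backdates the start time by that saved amount, so elapsed time is computed from Now on query without ticking.
; Starting from Stopping begins a fresh count.
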(fn `GetElapsedTime`
  (returns (Time :type "Timespan Structure"))
  (switch `/Game/Blueprints/BP_TimerStateEnum` (`self.CurrentState`)
    (:`NewEnumerator0`
      (return))
    (:`NewEnumerator1`
      (return (- (`KismetMathLibrary.Now`) (`self.StartTime`))))
    (:`NewEnumerator2`
      (return (`self.ElapsedTime`)))))

(fn `Pause`
  (switch `/Game/Blueprints/BP_TimerStateEnum` (`self.CurrentState`)
    (:`NewEnumerator1`
      (set `self.ElapsedTime` (- (`KismetMathLibrary.Now`) (`self.StartTime`)))
      (set `self.CurrentState` "NewEnumerator2"))))

(fn `Start`
  (switch `/Game/Blueprints/BP_TimerStateEnum` (`self.CurrentState`)
    (:`NewEnumerator0`
      (set `self.StartTime` (`KismetMathLibrary.Now`))
      (set `self.CurrentState` "NewEnumerator1"))
    (:`NewEnumerator2`
      (set `self.StartTime` (- (`KismetMathLibrary.Now`) (`self.ElapsedTime`)))
      (set `self.CurrentState` "NewEnumerator1"))))

(fn `Stop`
  (switch `/Game/Blueprints/BP_TimerStateEnum` (`self.CurrentState`)
    (:`NewEnumerator1`
      _)
    (:`NewEnumerator2`
      _))
  (set `self.CurrentState` "NewEnumerator0"))