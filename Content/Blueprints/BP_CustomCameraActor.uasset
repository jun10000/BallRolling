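; BP_CustomCameraActor is a camera actor that glides smoothly to a requested world location.
; MoveLocation stores the target and interpolation speed and starts the move, while SetInterpSpeed changes the speed separately.
; Tick applies VInterpTo while moving, then stops and fires OnMoveFinished once the actor is within tolerance of the target.
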(event `self.ReceiveBeginPlay`
  (set `self.DesiredLocation` (`self.K2_GetActorLocation`)))

(event `self.ReceiveTick`
  (params (DeltaSeconds :type "Float (single-precision)"))
  (if (`self.IsMoving`)
    (`self.K2_SetActorLocation` (`KismetMathLibrary.VInterpTo` (`self.K2_GetActorLocation`) (`self.DesiredLocation`) DeltaSeconds (`self.CurrentInterpSpeed`)))
    (if (== (`self.K2_GetActorLocation`) (`self.DesiredLocation`) :`ErrorTolerance` (`self.MoveLocationTolerance`))
      (set `self.IsMoving` false)
      (`self.OnMoveFinished`))))

(fn `MoveLocation`
  (params (NewLocation :type "Vector Structure") (Speed :type "Float (single-precision)"))
  (set `self.DesiredLocation` NewLocation)
  (set `self.CurrentInterpSpeed` Speed)
  (set `self.IsMoving` true))

(fn `SetInterpSpeed`
  (params (Speed :type "Float (single-precision)"))
  (set `self.CurrentInterpSpeed` Speed))

(fn `UserConstructionScript`)