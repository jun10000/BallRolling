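; Ball actor that offers both engine physics, toggled on its mesh, and a hand-written motion step, plus a goal particle effect.
; The manual step applies gravity, sweeps the actor, then mirrors velocity on impact with Z restitution and vertical-speed-scaled horizontal friction, spending the leftover frame time.
; Speed-based rolling sound logic exists, but its timer setup and hit flag are disconnected, so it never runs.
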(event `self.ReceiveBeginPlay`)

(event `Event_Timer`
  (if (`self.IsHit`)
    (`AudioComponent.Play` (`self.RollingSound`) 0.0)
    (set `self.IsHit` false))
  (`AudioComponent.SetVolumeMultiplier` (`self.RollingSound`) (`KismetMathLibrary.FClamp` (/ (`KismetMathLibrary.VSizeXY` (`self.GetVelocity`)) 1000.0))))

(event `self.ReceiveHit`
  (params (MyComp :type "PrimitiveComponent Object Reference") (Other :type "Actor Object Reference") (OtherComp :type "PrimitiveComponent Object Reference") (bSelfMoved :type Boolean) (HitLocation :type "Vector Structure") (HitNormal :type "Vector Structure") (NormalImpulse :type "Vector Structure") (Hit :type "HitResult Structure (by ref)")))

(fn `PlayGoalParticle`
  (bind _goalparticle (`self.GoalParticle`))
  (`SceneComponent.K2_SetWorldRotation` :`self` _goalparticle)
  (`ActorComponent.Activate` _goalparticle false))

(fn `SetSimulationEnable`
  (params (IsEnable :type Boolean))
  (`PrimitiveComponent.SetSimulatePhysics` (`self.StaticMeshComponent`) IsEnable))

(fn `TickSelfPhysicalSimulation`
  (params (DeltaSeconds :type "Float (single-precision)"))
  ;[1 1 1] 重力を速度に適用
  (set `self.CurrentVelocity` (+ (* (`self.Gravity`) DeltaSeconds) (`self.CurrentVelocity`)))
  (bind _sweephitresult (`self.K2_AddActorWorldOffset` (* (`self.CurrentVelocity`) DeltaSeconds) true))
  (bind (_bblockinghit _binitialoverlap _time _distance _location _impactpoint _normal) (`GameplayStatics.BreakHitResult` _sweephitresult))
  (if _bblockinghit
    (bind _returnvalue (`KismetMathLibrary.MirrorVectorByNormal` (`self.CurrentVelocity`) _normal))
    (bind _z (.z _returnvalue))
    (bind _returnvalue_2 (`KismetMathLibrary.VSizeXY` _returnvalue))
    (bind _returnvalue_3 (- _returnvalue_2 (`KismetMathLibrary.Abs` (* _z (`self.Friction`)))))
    (bind _returnvalue_4 (`KismetMathLibrary.SafeDivide` (`KismetMathLibrary.SelectFloat` _returnvalue_3 0.0 (> _returnvalue_3 0.0)) _returnvalue_2))
    ;[1 1 1] 速度を反射させる
    (set `self.CurrentVelocity` (`KismetMathLibrary.MakeVector` (* (.x _returnvalue) _returnvalue_4) (* (.y _returnvalue) _returnvalue_4) (* _z (`self.Restitution`))))
    (`self.K2_AddActorWorldOffset` (* (`self.CurrentVelocity`) (* DeltaSeconds (- 1.0 _time))) true)))

(fn `UserConstructionScript`)