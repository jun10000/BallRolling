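; One-shot trigger volume that activates bonus time spawners when the ball enters it.
; The first overlap by a BP_BallActor plays a 2D cat meow sound and calls Trig on every entry in the Spawners array.
; The construction script sizes the box from TriggerScale and raises it by its half-height, so its base sits at the actor's origin.
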(event `self.ReceiveActorBeginOverlap`
  (params (OtherActor :type "Actor Object Reference"))
  (cast `/Game/Blueprints/BP_BallActor` OtherActor)
  (`/Engine/EditorBlueprintResources/StandardMacros.DoOnce` false
    (:`Completed`
      (`/Game/Blueprints/BP_FunctionLibrary.PlaySound2D` "/Game/Sounds/SC_リアルな猫の鳴き声.SC_リアルな猫の鳴き声")
      (for _array_element (`self.Spawners`)
        (`/Game/Blueprints/IF_Triggerable.Trig` _array_element)))))

(fn `UserConstructionScript`
  (bind _returnvalue (* (`self.TriggerScale`) 50.0))
  (`BoxComponent.SetBoxExtent` (`self.BoxTrigger`) (`KismetMathLibrary.Conv_DoubleToVector` _returnvalue) true)
  (`SceneComponent.K2_SetRelativeLocation` (`self.BoxTrigger`) (`KismetMathLibrary.MakeVector` 0.0 0.0 _returnvalue) false false))