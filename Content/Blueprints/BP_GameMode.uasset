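; BP_GameMode is a game mode providing shared helpers for level flow, widgets, music, timing, version text and quitting.
; It advances through numbered stages via a GameInstance index, wrapping back to the title level.
; Widgets are cached by class and BGM uses one persistent audio component, both held on the GameInstance to outlive level changes.
; Total time is a lazily created timer's elapsed time minus bonus times tallied by value.
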(fn `AddBonusTime`
  (params (Time :type "Timespan Structure"))
  (bind _bonustimes (`self.BonusTimes`))
  (`BlueprintMapLibrary.Map_Add` _bonustimes Time (+ (`BlueprintMapLibrary.Map_Find` _bonustimes Time) 1)))

(fn `ExitGame`
  (`KismetSystemLibrary.QuitGame` null "Quit"))

(fn `GetElapsedTime`
  (returns (ReturnValue :type "Timespan Structure"))
  (return (`/Game/Blueprints/BP_Timer.GetElapsedTime` (`/Game/Blueprints/BP_FunctionLibrary.GetTimer`))))

(fn `GetTimer`
  (returns (Timer :type "/Game/Blueprints/BP_Timer Object Reference"))
  (bind _timer (`self.Timer`))
  (`/Engine/EditorBlueprintResources/StandardMacros.IsValid` _timer
    (:`Is Valid`
      (return _timer))
    (:`Is Not Valid`
      (bind _returnvalue (`|GenericCreateObject` "/Game/Blueprints/BP_Timer.BP_Timer_C"))
      (bind _output_get (set `self.Timer` _returnvalue))
      (return _output_get))))

(fn `GetTotalBonusTime`
  (returns (ReturnValue :type "Timespan Structure"))
  (locals (CurrentTotal :type "Timespan Structure"))
  (bind _bonustimes (`self.BonusTimes`))
  (bind _keys (`BlueprintMapLibrary.Map_Keys` _bonustimes))
  (for _array_element _keys
    (set `local.CurrentTotal` (+ (`local.CurrentTotal`) (* _array_element (`BlueprintMapLibrary.Map_Find` _bonustimes _array_element)))))
  (return (`local.CurrentTotal`)))

(fn `GetTotalTime`
  (returns (Time :type "Timespan Structure"))
  (return (- (`self.GetElapsedTime`) (`self.GetTotalBonusTime`))))

(fn `GetVersionText`
  (returns (Version :type Text))
  (return (`KismetTextLibrary.Conv_StringToText` (`KismetStringLibrary.JoinStringArray` (`/Game/Blueprints/BP_FunctionLibrary.ToStringArray (IntegerArray)` (`self.Version`)) "."))))

(fn `GetWidget`
  (params (Class :type "/Game/Widgets/W_Base Class Reference"))
  (returns (ReturnValue :type "/Game/Widgets/W_Base Object Reference"))
  (bind _widgets (`/Game/Blueprints/BP_GameInstance.Widgets` (`/Game/Blueprints/BP_FunctionLibrary.GetMyGameInstance`)))
  (bind (_value _returnvalue) (`BlueprintMapLibrary.Map_Find` _widgets Class))
  (if _returnvalue
    (return _value)
    (else
      (bind _returnvalue_2 (`|CreateWidget` Class))
      (`BlueprintMapLibrary.Map_Add` _widgets Class _returnvalue_2)
      (return _returnvalue_2))))

(fn `MoveToNextLevel`
  (bind _output_get (set `/Game/Blueprints/BP_GameInstance.CurrentLevelIndex` (mod (+ (`/Game/Blueprints/BP_GameInstance.CurrentLevelIndex` (`/Game/Blueprints/BP_FunctionLibrary.GetMyGameInstance`)) 1) (`self.LevelCount`)) (`/Game/Blueprints/BP_FunctionLibrary.GetMyGameInstance`)))
  (if (== _output_get 0)
    (`GameplayStatics.OpenLevelBySoftObjectPtr` "/Game/Maps/LV_Title.LV_Title")
    (else
      (`GameplayStatics.OpenLevel` (`KismetStringLibrary.Conv_StringToName` (`KismetStringLibrary.Concat_StrStr` "LV_Stage" (`/Game/Blueprints/BP_FunctionLibrary.GetZeroFilledString` _output_get)))))))

(fn `PlayBGM`
  (params (BGM :type "SoundBase Object Reference") (ID :type Integer) (Part :type Integer) (OnFinish :type "Delegate (by ref)"))
  (bind _audioplayer (`/Game/Blueprints/BP_GameInstance.AudioPlayer` (`/Game/Blueprints/BP_FunctionLibrary.GetMyGameInstance`)))
  (`/Engine/EditorBlueprintResources/StandardMacros.IsValid` _audioplayer
    (:`Is Valid`
      (if (`AudioComponent.IsPlaying` _audioplayer)
        (if (not (== (`AudioComponent.Sound` _audioplayer) BGM))
          (clear `AudioComponent.OnAudioFinished` _audioplayer :!label _label)
          (add `AudioComponent.OnAudioFinished` _audioplayer OnFinish)
          (`AudioParameterControllerInterface.SetIntParameter` _audioplayer "id" ID)
          (`AudioParameterControllerInterface.SetIntParameter` _audioplayer "part" Part)
          (`AudioComponent.SetSound` _audioplayer BGM)
          (`AudioComponent.Play` _audioplayer 0.0))
        (else
          (goto _label))))
    (:`Is Not Valid`
      (bind _returnvalue (`GameplayStatics.SpawnSound2D` BGM 1.0 1.0 0.0 null true false))
      (bind _output_get (set `/Game/Blueprints/BP_GameInstance.AudioPlayer` _returnvalue (`/Game/Blueprints/BP_FunctionLibrary.GetMyGameInstance`)))
      (clear `AudioComponent.OnAudioFinished` _output_get)
      (add `AudioComponent.OnAudioFinished` _output_get OnFinish)
      (`AudioParameterControllerInterface.SetIntParameter` _output_get "id" ID)
      (`AudioParameterControllerInterface.SetIntParameter` _output_get "part" Part))))

(fn `SetBGM`
  (params (BGM :type "SoundBase Object Reference") (ID :type Integer) (Part :type Integer) (OnFinish :type "Delegate (by ref)"))
  (`/Engine/EditorBlueprintResources/StandardMacros.IsValid` BGM
    (:`Is Valid`
      (`self.PlayBGM` BGM ID Part OnFinish))
    (:`Is Not Valid`
      (`self.StopBGM`))))

(fn `StopBGM`
  (bind _audioplayer (`/Game/Blueprints/BP_GameInstance.AudioPlayer` (`/Game/Blueprints/BP_FunctionLibrary.GetMyGameInstance`)))
  (`/Engine/EditorBlueprintResources/StandardMacros.IsValid` _audioplayer
    (:`Is Valid`
      (if (`AudioComponent.IsPlaying` _audioplayer)
        (`AudioComponent.Stop` _audioplayer)))))

(fn `UserConstructionScript`)