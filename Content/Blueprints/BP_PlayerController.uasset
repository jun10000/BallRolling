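; Player controller for a ball game where input tilts the stage, with rotation clamped per step and by maximum angle.
; Init sets the view target and stage, and input modes swap Enhanced Input contexts while remembering the previous one.
; It tracks balls up to a limit and destroys them on reset.
; Level sequences play in skippable Video mode, then restore input and fire a completion callback.
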(event `self.ReceiveBeginPlay`
  (`EnhancedInputSubsystemInterface.AddMappingContext` (pcsubsystem `EnhancedInputLocalPlayerSubsystem` self) "/Game/Inputs/IMC_Default.IMC_Default" 0 (struct)))

(event `EnhancedInput|/Game/Inputs/IA_Tilt`
  (params (ActionValue :type "Vector2D Structure") (ElapsedSeconds :type "Float (double-precision)") (TriggeredSeconds :type "Float (double-precision)") (InputAction :type "InputAction Object Reference" :default "/Game/Inputs/IA_Tilt.IA_Tilt"))
  (bind (_x _y) (`KismetMathLibrary.BreakVector2D` (* ActionValue (`self.MouseSensitivity`))))
  (:`Triggered`
    (`self.TiltStage` (`KismetMathLibrary.MakeRotator` _x (* _y -1.0)))))

(event `EnhancedInput|/Game/Inputs/IA_Reset`
  (params (ActionValue :type Boolean) (ElapsedSeconds :type "Float (double-precision)") (TriggeredSeconds :type "Float (double-precision)") (InputAction :type "InputAction Object Reference" :default "/Game/Inputs/IA_Reset.IA_Reset"))
  (:`Started`
    (for _array_element (`self.BallActors`)
      (`/Game/Blueprints/BP_ActorMacroLibrary.IsActorValid` _array_element
        (:`IsValid`
          (`self.K2_DestroyActor` _array_element))))))

(event `EnhancedInput|/Game/Inputs/IA_Exit`
  (params (ActionValue :type Boolean) (ElapsedSeconds :type "Float (double-precision)") (TriggeredSeconds :type "Float (double-precision)") (InputAction :type "InputAction Object Reference" :default "/Game/Inputs/IA_Exit.IA_Exit"))
  (:`Started`
    (`/Game/Blueprints/BP_GameMode.ExitGame` (`/Game/Blueprints/BP_FunctionLibrary.GetMyGameMode`))))

(event `EnhancedInput|/Game/Inputs/IA_SkipVideo`
  (params (ActionValue :type Boolean) (ElapsedSeconds :type "Float (double-precision)") (TriggeredSeconds :type "Float (double-precision)") (InputAction :type "InputAction Object Reference" :default "/Game/Inputs/IA_SkipVideo.IA_SkipVideo"))
  (:`Started`
    (`self.FinishLevelSequence`)))

(fn `AddBall`
  (params (NewBall :type "/Game/Blueprints/BP_BallActor Object Reference (by ref)"))
  (returns (IsSuccess :type Boolean))
  (`self.UpdateBallActorArray`)
  (if (< (`KismetArrayLibrary.Array_Length` (`self.BallActors`)) (`self.MaxBallCount`))
    (`KismetArrayLibrary.Array_AddUnique` (`self.BallActors`) NewBall)
    (return true)
    (else
      (return false))))

(fn `FinishLevelSequence`
  (bind _lsactor (`self.LSActor`))
  (bind _sequenceplayer (`LevelSequenceActor.SequencePlayer` _lsactor))
  (`/Game/Blueprints/BP_ActorMacroLibrary.IsActorValid` _lsactor
    (:`IsValid`
      (if (`MovieSceneSequencePlayer.IsPlaying` _sequenceplayer)
        (`MovieSceneSequencePlayer.GoToEndAndStop` _sequenceplayer)))))

(fn `GetBall`
  (params (Index :type Integer))
  (returns (ReturnValue :type "/Game/Blueprints/BP_BallActor Object Reference") (IsSuccess :type Boolean))
  (bind _ballactors (`self.BallActors`))
  (if (`KismetArrayLibrary.Array_IsValidIndex` _ballactors Index)
    (return (`|GetArrayItem` _ballactors Index) true)
    (else
      (return null false))))

(fn `GetIMCFromInputMode`
  (params (InputMode :type "/Game/Blueprints/BP_ControllerInputModeEnum Enum" :default "NewEnumerator2"))
  (returns (IMC :type "InputMappingContext Object Reference"))
  (switch `/Game/Blueprints/BP_ControllerInputModeEnum` InputMode
    (:`NewEnumerator2`
      _)
    (:`NewEnumerator0`
      (return "/Game/Inputs/IMC_Video.IMC_Video"))
    (:`NewEnumerator1`
      (return "/Game/Inputs/IMC_Game.IMC_Game"))
    (:`NewEnumerator3`
      _))
  (return null))

(fn `GetInputMode`
  (returns (InputMode :type "/Game/Blueprints/BP_ControllerInputModeEnum Enum"))
  (return (`self.InputMode`)))

(fn `Init`
  (params (ViewActor :type "Actor Object Reference") (StageActor :type "Actor Object Reference"))
  (bind _output_get (set `self.ViewActor` ViewActor))
  (`self.SetViewTargetWithBlend` _output_get 0.0 "VTBlend_PreBlended")
  (set `self.StageActor` StageActor)
  (`self.SetInputMode` (`self.InputMode`)))

(fn `PlayLevelSequence`
  (params (LSActor :type "LevelSequenceActor Object Reference") (OnComplete :type "Delegate (by ref)"))
  (bind _output_get (set `self.LSActor` LSActor))
  (`/Game/Blueprints/BP_ActorMacroLibrary.IsActorValid` _output_get
    (:`IsValid`
      (set `self.IsLevelSequenceComplete` false)
      (clear `self.OnLevelSequenceComplete`)
      (add `self.OnLevelSequenceComplete` OnComplete)
      (bind _sequenceplayer (`LevelSequenceActor.SequencePlayer` _output_get))
      (clear `MovieSceneSequencePlayer.OnFinished` _sequenceplayer)
      (clear `MovieSceneSequencePlayer.OnStop` _sequenceplayer)
      (clear `MovieSceneSequencePlayer.OnPause` _sequenceplayer)
      (add `MovieSceneSequencePlayer.OnFinished` _sequenceplayer (`|CreateDelegate` :!event `PlayLevelSequence_OnComplete`))
      (add `MovieSceneSequencePlayer.OnStop` _sequenceplayer (`|CreateDelegate` :!event `PlayLevelSequence_OnComplete`))
      (add `MovieSceneSequencePlayer.OnPause` _sequenceplayer (`|CreateDelegate` :!event `PlayLevelSequence_OnComplete`))
      (`self.SetInputMode` "NewEnumerator0")
      (`MovieSceneSequencePlayer.Play` _sequenceplayer))))

(fn `PlayLevelSequence_OnComplete`
  (if (not (`self.IsLevelSequenceComplete`))
    (set `self.IsLevelSequenceComplete` true)
    (`self.RestoreInputMode`)
    (`self.OnLevelSequenceComplete`)))

(fn `RestoreInputMode`
  (`self.SetInputMode` (`self.PrevInputMode`)))

(fn `SetInputMode`
  (params (Mode :type "/Game/Blueprints/BP_ControllerInputModeEnum Enum" :default "NewEnumerator1"))
  (bind _returnvalue (pcsubsystem `EnhancedInputLocalPlayerSubsystem` self))
  (`EnhancedInputSubsystemInterface.RemoveMappingContext` _returnvalue (`self.GetIMCFromInputMode` (`self.InputMode`)) (struct))
  (`EnhancedInputSubsystemInterface.AddMappingContext` _returnvalue (`self.GetIMCFromInputMode` Mode) 0 (struct))
  (set `self.PrevInputMode` (`self.InputMode`))
  (bind _output_get (set `self.InputMode` Mode))
  (if (`|EnumEquality` _output_get "NewEnumerator3")
    (`WidgetBlueprintLibrary.SetInputMode_UIOnlyEx` self null)
    (else
      (`WidgetBlueprintLibrary.SetInputMode_GameOnly` self))))

(fn `SetLevelSequence`
  (params (LSActor :type "LevelSequenceActor Object Reference"))
  (set `self.LSActor` LSActor))

(fn `TiltStage`
  (params (AddRotator :type "Rotator Structure"))
  (bind _maxtiltspeed (`self.MaxTiltSpeed`))
  (bind _maxtiltangle (`self.MaxTiltAngle`))
  (bind _stageactor (`self.StageActor`))
  (bind _returnvalue (* _maxtiltangle -1.0))
  (bind _returnvalue_2 (* _maxtiltspeed -1.0))
  (`/Game/Blueprints/BP_ActorMacroLibrary.IsActorValid` _stageactor
    (:`IsValid`
      (`self.K2_SetActorRelativeRotation` _stageactor (`/Game/Blueprints/BP_FunctionLibrary.ClampRotator` (`KismetMathLibrary.ComposeRotators` (`self.K2_GetActorRotation` _stageactor) (`/Game/Blueprints/BP_FunctionLibrary.ClampRotator` AddRotator _returnvalue_2 _maxtiltspeed _returnvalue_2 _maxtiltspeed)) _returnvalue _maxtiltangle _returnvalue _maxtiltangle) true false))))

(fn `UpdateBallActorArray`
  (bind _ballactors (`self.BallActors`))
  (for _array_element _ballactors
    (`/Game/Blueprints/BP_ActorMacroLibrary.IsActorValid` _array_element
      (:`IsNotValid`
        (`KismetArrayLibrary.Array_RemoveItem` _ballactors _array_element)))))

(fn `UserConstructionScript`)