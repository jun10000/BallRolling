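; BP_BonusTimeSpawner is a placeable spawner for BP_BonusTimeActor, passing it a configurable BonusSeconds value.
; The construction script scales X and Y by DiameterScale, and spawned actors receive that scale through the spawner's transform.
; Spawn creates a new actor only when the tracked one is invalid, then attaches it to the spawner's parent, keeping world transform.
; The event graph is empty, so Spawn relies on external callers.
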(fn `Spawn`
  (`/Game/Blueprints/BP_ActorMacroLibrary.IsActorValid` (`self.CurrentSpawnedActor`)
    (:`IsNotValid`
      (bind _returnvalue (`|SpawnActorFromClass` "/Game/Blueprints/BP_BonusTimeActor.BP_BonusTimeActor_C" (`self.GetTransform`) "Undefined" "MultiplyWithRoot" null (`self.BonusSeconds`) null))
      (`self.K2_AttachToActor` _returnvalue (`self.GetAttachParentActor`) "None" "KeepWorld" "KeepWorld" "KeepWorld" true)
      (set `self.CurrentSpawnedActor` _returnvalue))))

(fn `UserConstructionScript`
  (bind _diameterscale (`self.DiameterScale`))
  (`self.SetActorScale3D` (`KismetMathLibrary.MakeVector` _diameterscale _diameterscale 1.0)))